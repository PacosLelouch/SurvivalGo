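; BP_GoPlayingPlayerState is a player state Blueprint that owns the local player's main playing HUD.
; When the override player index replicates, it rebuilds the HUD, removing any old BPW_PlayingMain and creating a new one only for a local player controller.
; An action value notify event pushes current and total action values into the HUD's PlayerInfo widget.
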(event `self.OnRep_OverridePlayerIndex`
  ;[1 1 1] OnRep
  (`parent.OnRep_OverridePlayerIndex`)
  (`self.InitUI`))

(event `InitUI`
  (bind _returnvalue (`self.GetOwningController` "/Script/Engine.PlayerController"))
  (bind _playingmainui (`self.PlayingMainUI`))
  ;[1 1 1] User Interface
  (`|ExecutionSequence`
    (:`then_0`
      (`/Engine/EditorBlueprintResources/StandardMacros.IsValid` _playingmainui
        (:`Is Valid`
          (`Widget.RemoveFromParent` _playingmainui)
          (set `self.PlayingMainUI` null))))
    (:`then_1`
      (`/Engine/EditorBlueprintResources/StandardMacros.IsValid` _returnvalue
        (:`Is Valid`
          (if (`Controller.IsLocalPlayerController` _returnvalue)
            (bind _returnvalue_2 (`|CreateWidget` "/Game/GameCore/Blueprints/UI/PlayingMain/BPW_PlayingMain.BPW_PlayingMain_C" _returnvalue))
            (bind _output_get (set `self.PlayingMainUI` _returnvalue_2))
            (`/Engine/EditorBlueprintResources/StandardMacros.IsValid` _output_get
              (:`Is Valid`
                (`UserWidget.AddToViewport` _output_get 0)))))))))

(event `ActionValueNotifierInterface.NotifyActionValueViewToUpdate`
  (bind _playingmainui (`self.PlayingMainUI`))
  (bind _playerinfo (`/Game/GameCore/Blueprints/UI/PlayingMain/BPW_PlayingMain.PlayerInfo` _playingmainui))
  ;[1 1 1] User Interface
  (`/Engine/EditorBlueprintResources/StandardMacros.IsValid` _playingmainui
    (:`Is Valid`
      (`/Engine/EditorBlueprintResources/StandardMacros.IsValid` _playerinfo
        (:`Is Valid`
          (`/Game/GameCore/Blueprints/UI/PlayingMain/BPW_PlayerInfo.UpdateActionValue` _playerinfo (`self.CurrentActionValue`) (`self.TotalActionValue`)))))))

(fn `UserConstructionScript`)