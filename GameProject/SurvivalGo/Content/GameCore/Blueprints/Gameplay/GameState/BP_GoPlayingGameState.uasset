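; Playing-phase game state Blueprint for a turn-based Go game, extending a parent game state that owns round, turn and phase data.
; On BeginPlay it passes the Go game instance to InitPPMPC.
; When a move to the next phase is triggered, it waits briefly, calls the parent's phase handling, then prints the round, player turn and phase for debugging.
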(event `self.ReceiveBeginPlay`
  (bind _asgo_game_instance (cast `GoGameInstance` (`GameplayStatics.GetGameInstance`)))
  (`/Game/GameCore/Blueprints/Functions/BPFL_InitLibrary.InitPPMPC` _asgo_game_instance))

(event `self.DealWithMoveToNextPhase`
  (`KismetSystemLibrary.PrintString` "Ready to move to next phase.")
  (`KismetSystemLibrary.Delay` 1.0)
  (`parent.DealWithMoveToNextPhase`)
  (`KismetSystemLibrary.PrintString` (`KismetStringLibrary.Concat_StrStr` "Phase: " (`KismetStringLibrary.Conv_IntToString` (`self.Round`)) ", " (`KismetStringLibrary.Conv_IntToString` (`self.PlayerTurn`)) ", " (`|GetEnumeratorNameAsString` (`self.RoundPhase`)))))

(fn `UserConstructionScript`)