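; Player controller for turn-based chess-piece play on a block map, accepting click or touch during the local player's Action phase.
; Traces select an owned piece, caching blocks within its action-point range, then move it or attack a target.
; Moves and attacks pass through Server events to MapBuilder multicasts, while a transaction state gates input.
; A looping timer retries PlayerState and GameState setup, then binds phase changes that clear selection off-turn.
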(event `SwitchTransactionState`
  (params (TargetTransactionState :type "EOperationTransactionState Enum" :default "NotInTransaction"))
  (bind _output_get (set `self.OperationTransactionState` TargetTransactionState))
  (if (not (`GameplayUtilLibrary.IsInTransaction` _output_get))
    (`self.ClearSelectedChess`)))

(event `ClearSelectedChess`
  (bind _selectedchess (`self.SelectedChess`))
  ;[1 1 1] Select Owned Chess
  (`/Engine/EditorBlueprintResources/StandardMacros.IsValid` _selectedchess
    (:`Is Valid`
      (set `GoChessPawn.bIsLocallySelected` false _selectedchess)
      (clear `GoChessPawn.OnChangeOperationTransactionDelegate` (`self.SelectedChess`))
      (set `self.SelectedChess` null)
      (`BlueprintMapLibrary.Map_Clear` (`self.CurrentMovableBlocks`))
      (set `self.OperationTransactionState` "NotInTransaction") ; In case.
    )))

(event `self.ReceiveBeginPlay`
  ;[1 1 1] Initialize
  (bind _returnvalue (`KismetSystemLibrary.K2_SetTimerDelegate` (delegate `InitPC`) 0.2 true)))

(event `SelectOwnedChess`
  (params (ChessToSelect :type "GoChessPawn Object Reference"))
  (bind _selectedchess (`self.SelectedChess`))
  (bind (_value _returnvalue) (`BlueprintMapLibrary.Map_Find` (`GoMapBuilder.BlockData` (`self.GetMapBuilder`)) (`MapElementLibrary.ToBlockCoordinate` (`GoChessPawn.Coordinate` _selectedchess))))
  ;[1 1 1] Select Owned Chess
  (`|ExecutionSequence`
    (:`then_0`
      (`self.ClearSelectedChess`))
    (:`then_1`
      (bind _output_get (set `self.SelectedChess` ChessToSelect))
      (set `GoChessPawn.bIsLocallySelected` true _output_get)
      (if _returnvalue
        (bind _outtargets (message `MapSourceInterface.GetAdjacentsWithDistance` (`self.GetMapBuilder`) _value (/ (`GoPlayingPlayerState.CurrentActionValue` (`self.GoPlayingPS`)) (`GoChessPawn.MoveActionCost` _selectedchess)) "Movable" false))
        (bind _dst (`MapElementLibrary.InterfaceToBlock_ObjIntMap` _outtargets))
        (set `self.CurrentMovableBlocks` _dst)))
    (:`then_2`
      (add `GoChessPawn.OnChangeOperationTransactionDelegate` (`self.SelectedChess`) (`|CreateDelegate` :!event `SwitchTransactionState`)))))

(event `InitPC`
  ;[1 1 1] Initialize
  (bind _asgo_playing_player_state (cast `GoPlayingPlayerState` (`self.PlayerState`)))
  (set `self.GoPlayingPS` _asgo_playing_player_state)
  (bind _asgo_playing_game_state (cast `GoPlayingGameState` (`GameplayStatics.GetGameState`)))
  (bind _output_get (set `self.GoPlayingGS` _asgo_playing_game_state))
  (if (and (`KismetSystemLibrary.IsValid` (`self.GoPlayingGS`)) (`KismetSystemLibrary.IsValid` (`self.GoPlayingPS`)))
    (add `GoPlayingGameState.PostMoveToNextPhaseDelegate` _asgo_playing_game_state (delegate `NotifyMoveToNextPhase`))
    (add `GoPlayingGameState.PostMoveToNextPhaseDelegate` _output_get (delegate `NotifyMoveToNextPhase`))
    (`KismetSystemLibrary.K2_PauseTimerHandle` (stale `self.ReceiveBeginPlay` _returnvalue))))

(event `NotifyMoveToNextPhase`
  (params (Round :type Integer) (PlayerTurn :type Integer) (RoundPhase :type "ERoundPhase Enum" :default "Unknown"))
  ;[1 1 1] Initialize
  (if (not (== (`GoPlayingPlayerState.GetPlayerIndex` (`self.GoPlayingPS`) true) PlayerTurn))
    (`self.ClearSelectedChess`)))

(event `InputTouch`
  (params (Location :type "Vector Structure") (FingerIndex :type "ETouchIndex Enum"))
  (bind _goplayinggs (`self.GoPlayingGS`))
  ;[1 1 1] Deal With Input
  (:`Released`
    (if (and (not (`GameplayUtilLibrary.IsInTransaction` (`self.OperationTransactionState`))) (and (== (`GoPlayingGameState.PlayerTurn` _goplayinggs) (`GoPlayingPlayerState.GetPlayerIndex` (`self.GoPlayingPS`) true)) (`|EnumEquality` (`GoPlayingGameState.RoundPhase` _goplayinggs) "Action"))) :!label _label
      (`|ExecutionSequence`
        (:`then_1`
          (bind _outhitresult (`self.TraceSingleGetHitResult`))
          (bind (_targetobstacle _bownchess _returnvalue) (`self.TraceObstacle` _outhitresult))
          (if _returnvalue
            (`|ExecutionSequence`
              (:`then_0`
                (if _bownchess
                  (bind _asgo_chess_pawn (cast `GoChessPawn` _targetobstacle))
                  (`self.SelectOwnedChess` _asgo_chess_pawn)
                  (else
                    (bind _asmap_obstacle_interface (cast `MapObstacleInterface` _targetobstacle))
                    (`self.MakeAttack` _asmap_obstacle_interface))))
              (:`then_1`
                (`KismetSystemLibrary.PrintString` (`KismetStringLibrary.Concat_StrStr` "Traced [" (`KismetSystemLibrary.GetDisplayName` _targetobstacle) "], OwnChess: " (`KismetStringLibrary.Conv_BoolToString` _bownchess)) true true (struct :`G` 0.66 :`B` 1.0 :`A` 1.0) 5.0)))
            (else
              (bind (_targetblock _returnvalue_2) (`self.TraceBlock` _outhitresult))
              (if _returnvalue_2
                (`|ExecutionSequence`
                  (:`then_0`
                    (if (`.ReturnValue` (`BlueprintMapLibrary.Map_Find` (`self.CurrentMovableBlocks`) _targetblock))
                      (`self.MoveChessTo` _targetblock)
                      (else
                        (bind _coordinate_coordinate (break `MapCoordinate` (`MapBlock.Coordinate` _targetblock)))
                        (`KismetSystemLibrary.PrintString` (`KismetStringLibrary.Concat_StrStr` "Traced Block [" (`KismetStringLibrary.Conv_IntVectorToString` _coordinate_coordinate) "], Type: " (`|GetEnumeratorNameAsString` (`MapBlock.BlockType` _targetblock)) "(Too Far Away)"))))))
                (else
                  (`self.ClearSelectedChess`)))))))
      (else
        (`KismetSystemLibrary.PrintString` "Not your turn or action phase." true true (struct :`R` 1.0 :`G` 0.851721 :`B` 0.108272 :`A` 1.0))))))

(event `Key|LeftMouseButton`
  (params (Key :type "Key Structure"))
  ;[1 1 1] Deal With Input
  (:`Released`
    (goto _label)))

(event `MoveChessTo`
  (params (TargetBlock :type "MapBlock Object Reference"))
  (bind _returnvalue (`self.GetMapBuilder`))
  (bind _selectedchess (`self.SelectedChess`))
  (bind _selectedchess_2 (`self.SelectedChess`))
  ;[1 1 1] Move Chess To
  (`/Engine/EditorBlueprintResources/StandardMacros.IsValid` _selectedchess_2
    (:`Is Valid`
      (if (and (`GoChessPawn.bIsLocallySelected` _selectedchess_2) (not (`GoChessPawn.IsChessMoving` _selectedchess_2)))
        (if (== (`BlueprintSetLibrary.Set_Length` (`MapBlock.Obstacles` TargetBlock)) 0)
          (`|ExecutionSequence`
            (:`then_0`
              (set `self.TempFromPosition` (`GoMapBuilder.GetPosition` _returnvalue (`GoChessPawn.Coordinate` _selectedchess_2)))
              (set `self.TempToPosition` (`GoMapBuilder.GetPosition` _returnvalue (`MapBlock.Coordinate` TargetBlock))))
            (:`then_1`
              (`self.UpdateChessMoveServer` (`GoChessPawn.OwningPlayerIndex` _selectedchess) (`GoChessPawn.ChessIndex` _selectedchess) (`GoMapBuilder.GetCoordinate` (`self.GetMapBuilder`) (`self.TempToPosition`) (`MapElementLibrary.GetPawnDirectionByRotator` (`KismetMathLibrary.Conv_VectorToRotator` (- (`self.TempToPosition`) (`self.TempFromPosition`)))))))))))))

(event `UpdateChessMoveServer`
  (params (PlayerIndex :type Integer) (ChessIndex :type Integer) (NewCoordinate :type "MapCoordinate Structure (by ref)"))
  ;[1 1 1] Move Chess To
  (`GoMapBuilder.UpdateMapBuilderCoordinateInternalMulticast` (`self.GetMapBuilder`) PlayerIndex ChessIndex NewCoordinate))

(event `UpdateChessAttackChessServer`
  (params (FromPlayerIndex :type Integer) (FromChessIndex :type Integer) (ToPlayerIndex :type Integer) (ToChessIndex :type Integer))
  ;[1 1 1] Make Attack
  (`GoMapBuilder.UpdateChessAttackChessMulticast` (`self.GetMapBuilder`) FromPlayerIndex FromChessIndex ToPlayerIndex ToChessIndex))

(event `MakeAttack`
  (params (Target :type "MapObstacleInterface Interface"))
  (bind _selectedchess (`self.SelectedChess`))
  (bind _owningplayerindex (`GoChessPawn.OwningPlayerIndex` _selectedchess))
  (bind _chessindex (`GoChessPawn.ChessIndex` _selectedchess))
  ;[1 1 1] Make Attack
  (`/Engine/EditorBlueprintResources/StandardMacros.IsValid` _selectedchess
    (:`Is Valid`
      (if (>= (`GoPlayingPlayerState.CurrentActionValue` (`self.GoPlayingPS`)) (`GoChessPawn.AttackActionCost` _selectedchess))
        (bind _asgo_chess_pawn (cast `GoChessPawn` Target)
          (:`then`
            (`self.UpdateChessAttackChessServer` _owningplayerindex _chessindex (`GoChessPawn.OwningPlayerIndex` _asgo_chess_pawn) (`GoChessPawn.ChessIndex` _asgo_chess_pawn)))
          (:`CastFailed`
            (bind _asnon_player_obstacle (cast `NonPlayerObstacle` Target))
            (`self.UpdateChessAttackObstacleServer` _owningplayerindex _chessindex (`NonPlayerObstacle.ObstacleId` _asnon_player_obstacle))))))))

(event `UpdateChessAttackObstacleServer`
  (params (FromPlayerIndex :type Integer) (FromChessIndex :type Integer) (ToObstacleId :type Integer))
  ;[1 1 1] Make Attack
  (`GoMapBuilder.UpdateChessAttackObstacleMulticast` (`self.GetMapBuilder`) FromPlayerIndex FromChessIndex ToObstacleId))

(fn `UserConstructionScript`)