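; Game mode for a playing match that sets up players, the map and game phases.
; BeginPlay takes total and AI player counts from the game instance and loads map settings.
; Once all human players log in, delayed steps create AI players, assign player indices (marked test code), generate the scene and start the first phase.
; A debug-style Alt+M key advances phases, and map build completion prints a message.
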(event `self.K2_PostLogin`
  (params (NewPlayer :type "PlayerController Object Reference"))
  (bind _logincount (`self.LoginCount`))
  (`/Engine/EditorBlueprintResources/StandardMacros.IncrementInt` _logincount
    (:`  `
      (bind _asgo_playing_game_state (cast `GoPlayingGameState` (`GameplayStatics.GetGameState`)))
      (if (== _logincount (- (`GoPlayingGameState.TotalPlayer` _asgo_playing_game_state) (`GoPlayingGameState.AIPlayer` _asgo_playing_game_state)))
        (`KismetSystemLibrary.Delay` 0.2)
        (`|ExecutionSequence`
          (:`then_0`
            (`self.CreateAIPlayers`))
          (:`then_1`
            ;[1 1 1] TestCode
            (for (_array_element _array_index) (`GameStateBase.PlayerArray` _asgo_playing_game_state)
              (bind _asgo_playing_player_state (cast `GoPlayingPlayerState` _array_element))
              (bind _output_get (set `GoPlayingPlayerState.OverridePlayerIndex` _array_index _asgo_playing_player_state))
              (if (== _output_get 0)
                (`GoPlayingPlayerState.OnRep_OverridePlayerIndex` _asgo_playing_player_state))))
          (:`then_2`
            (set `self.bMapSettingsHaveLoaded` true)
            (`self.GenerateScene` (`MapSubsystem.MapSettings` (subsystem `MapSubsystem`))))
          (:`then_3`
            (`KismetSystemLibrary.Delay` 0.5)
            (`self.InitPhase`)))))))

(event `self.ReceiveBeginPlay`
  ;[1 1 1] TestCode
  (bind _asgo_game_instance (cast `GoGameInstance` (`GameplayStatics.GetGameInstance`)))
  (`self.InitPlayerNum` (`GoGameInstance.HostTotalPlayerNum` _asgo_game_instance) (`GoGameInstance.HostAIPlayerNum` _asgo_game_instance))
  (`self.LoadMapSettings` (`self.Settings Name`))
  (`self.EnableInput` (`GameplayStatics.GetPlayerController` 0)))

(event `Key|Alt+M`
  (params (Key :type "Key Structure"))
  ;[1 1 1] TestCode
  (:`Released`
    (`self.MoveToNextPhase`)))

(event `self.PostMapBuildComplete`
  (`|ExecutionSequence`
    (:`then_0`
      (`parent.PostMapBuildComplete`)
      (`KismetSystemLibrary.PrintString` "Map build complete."))))

(fn `UserConstructionScript`)