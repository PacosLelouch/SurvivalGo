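; Map builder Blueprint that generates the game map from settings, updates data from game state, and places obstacles and chess pawns.
; On BeginPlay it clears temp queues and polls on a looping timer until map settings are initialized, then builds and pauses the timer.
; Obstacle and pawn additions are queued and passed to the parent implementation by polling timers once block data count matches the settings.
; Older RetriggerableDelay retry loops remain disconnected.
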(event `self.ReceiveBeginPlay`
  (`self.ClearAllTemp`)
  (bind _returnvalue (`KismetSystemLibrary.K2_SetTimerDelegate` (delegate `InitMapBuilder`) 0.2 true)))

(event `InitMapBuilder`
  (if (`self.bIsMapSettingsInited`)
    (`|ExecutionSequence`
      (:`then_0`
        (`self.GenerateMapFromSettings`)
        (`self.UpdateDatasFromGameState`))
      (:`then_1`
        (`KismetSystemLibrary.K2_PauseTimerHandle` (stale `self.ReceiveBeginPlay` _returnvalue))))))

(event `self.AddObstacle`
  (params (Obstacle :type "Actor Object Reference") (Coordinate :type "MapCoordinate Structure (by ref)"))
  (`KismetArrayLibrary.Array_Add` (`self.TempObstacles`) Obstacle)
  (`KismetArrayLibrary.Array_Add` (`self.TempObstacleCoordinates`) Coordinate)
  (bind _returnvalue (`KismetSystemLibrary.K2_SetTimerDelegate` (delegate `TryToAddObstacle`) 0.2 true)))

(event `TryToAddObstacle`
  (bind _tempobstacleindex (`self.TempObstacleIndex`))
  (if (== (`KismetArrayLibrary.Array_Length` (`.BlockDataSettings` (break `MapSettings` (`self.InitMapSettings`)))) (`BlueprintMapLibrary.Map_Length` (`self.BlockData`)))
    (`|ExecutionSequence`
      (:`then_0`
        (`parent.AddObstacle` (`|GetArrayItem` (`self.TempObstacles`) _tempobstacleindex) (`|GetArrayItem` (`self.TempObstacleCoordinates`) _tempobstacleindex))
        (`/Engine/EditorBlueprintResources/StandardMacros.IncrementInt` (`self.TempObstacleIndex`)))
      (:`then_1`
        (`KismetSystemLibrary.K2_PauseTimerHandle` (stale `self.AddObstacle` _returnvalue))))))

(event `self.AddChessPawn`
  (params (ChessPawn :type "GoChessPawn Object Reference") (Coordinate :type "MapCoordinate Structure (by ref)"))
  (`KismetArrayLibrary.Array_Add` (`self.TempChesses`) ChessPawn)
  (`KismetArrayLibrary.Array_Add` (`self.TempChessCoordinates`) Coordinate)
  (bind _returnvalue (`KismetSystemLibrary.K2_SetTimerDelegate` (delegate `TryToAddChessPawn`) 0.2 true)))

(event `TryToAddChessPawn`
  (bind _tempchessindex (`self.TempChessIndex`))
  (if (== (`KismetArrayLibrary.Array_Length` (`.BlockDataSettings` (break `MapSettings` (`self.InitMapSettings`)))) (`BlueprintMapLibrary.Map_Length` (`self.BlockData`)))
    (`|ExecutionSequence`
      (:`then_0`
        (`parent.AddChessPawn` (`|GetArrayItem` (`self.TempChesses`) _tempchessindex) (`|GetArrayItem` (`self.TempChessCoordinates`) _tempchessindex))
        (`/Engine/EditorBlueprintResources/StandardMacros.IncrementInt` (`self.TempChessIndex`)))
      (:`then_1`
        (`KismetSystemLibrary.K2_PauseTimerHandle` (stale `self.AddChessPawn` _returnvalue))))))

(fn `ClearAllTemp`
  (`KismetArrayLibrary.Array_Clear` (`self.TempObstacles`))
  (`KismetArrayLibrary.Array_Clear` (`self.TempChesses`))
  (`KismetArrayLibrary.Array_Clear` (`self.TempObstacleCoordinates`))
  (`KismetArrayLibrary.Array_Clear` (`self.TempChessCoordinates`))
  (set `self.TempObstacleIndex` 0)
  (set `self.TempChessIndex` 0))

(fn `UserConstructionScript`)