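; BP_BreakableWall is a breakable wall obstacle that shows its health on a health bar.
; The NotifyHealthViewtoUpdate event passes current and initial total health to the HealthBar and prints a debug message with the wall's name.
; BeginPlay fires that event once to initialize the bar, and GetObstacleType exposes the wall's obstacle type.
; Damage and breaking logic are absent from these graphs.
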(event `HealthNotifierInterface.NotifyHealthViewToUpdate`
  ;[1 1 1] User Interface
  (`/Game/GameCore/Blueprints/UI/Floating/BP_HealthBarWidgetComponent.UpdateHealth` (`self.HealthBar`) (`self.CurrentHealth`) (`self.InitialTotalHealth`))
  (`KismetSystemLibrary.PrintString` (`KismetStringLibrary.Concat_StrStr` (`KismetSystemLibrary.GetDisplayName` self) " gets attack?")))

(event `self.ReceiveBeginPlay`
  (`HealthNotifierInterface.NotifyHealthViewToUpdate`))

(fn `GetObstacleType`
  (returns (ReturnValue :type "EObstacleType Enum"))
  (return (`self.ObstacleType`)))

(fn `UserConstructionScript`)