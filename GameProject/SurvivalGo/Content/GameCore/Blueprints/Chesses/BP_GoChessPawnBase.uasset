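; Base Blueprint for a board chess pawn, handling the visual side of moves, attacks and health display.
; ChessMovementComponent animates single (deprecated) and batch moves, which then clear selection and end the operation transaction.
; Attacks turn the pawn and joining chesses toward the target and play montages.
; After the attacker's montage, selection clears, the target's health view refreshes, and the authority calls delayed destroy-if-needed on the target.
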(event `self.ReceiveBeginPlay`
  ;[1 1 1] Initialize
  (`HealthNotifierInterface.NotifyHealthViewToUpdate`))

(event `self.MoveOnceInView`
  (params (FromTransform :type "Transform Structure (by ref)") (ToTransform :type "Transform Structure (by ref)"))
  ;[1 1 1] Move Once In View (Deprecated)
  (`parent.MoveOnceInView` FromTransform ToTransform)
  (`ChessMovementComponent.MoveActorOnce` (`self.ChessMovementComponent`) FromTransform ToTransform true -1.0 -1.0)
  (set `self.bIsLocallySelected` false)
  (`self.OnChangeOperationTransactionDelegate` "NotInTransaction"))

(event `self.MoveBatchInView`
  (params (FromTransform :type "Transform Structure (by ref)") (ToTransforms :type "Array of Transform Structure (by ref)"))
  ;[1 1 1] Move Batch In View
  (`parent.MoveBatchInView` FromTransform ToTransforms)
  (`ChessMovementComponent.MoveActorBatch` (`self.ChessMovementComponent`) FromTransform ToTransforms true -1.0 -1.0
    (:`AllCompleted`
      (set `self.bIsLocallySelected` false)
      (`self.OnChangeOperationTransactionDelegate` "NotInTransaction"))))

(event `HealthNotifierInterface.NotifyHealthViewToUpdate`
  ;[1 1 1] User Interface
  (`/Game/GameCore/Blueprints/UI/Floating/BP_HealthBarWidgetComponent.UpdateHealth` (`self.HealthBar`) (`self.CurrentHealth`) (`self.InitialTotalHealth`))
  (`KismetSystemLibrary.PrintString` (`KismetStringLibrary.Concat_StrStr` (`KismetSystemLibrary.GetDisplayName` self) " gets attack?")))

(event `self.AttackInView`
  (params (Target :type "MapObstacleInterface Interface (by ref)") (WithOtherChesses :type "Array of GoChessPawn Object Reference (by ref)"))
  (bind (_returnvalue_location _returnvalue_rotation _returnvalue_scale) (`KismetMathLibrary.BreakTransform` (`self.GetTransform`)))
  (bind _returnvalue (`MapSubsystem.GetMapBuilder` (subsystem `MapSubsystem`)))
  (bind _returnvalue_2 (`MapSubsystem.GetMapBuilder` (subsystem `MapSubsystem`)))
  ;[1 1 1] Attack In View
  (if (`self.CheckBeforeAttack` Target WithOtherChesses)
    (for _array_element WithOtherChesses
      (bind (_returnvalue_location_2 _returnvalue_rotation_2 _returnvalue_scale_2) (`KismetMathLibrary.BreakTransform` (`self.GetTransform` _array_element)))
      (`ChessMovementComponent.MoveActorOnce` (`GoChessPawn.ChessMovementComponent` _array_element) (`KismetMathLibrary.MakeTransform` _returnvalue_location_2 _returnvalue_rotation_2 _returnvalue_scale_2) (`KismetMathLibrary.MakeTransform` _returnvalue_location_2 (`KismetMathLibrary.Conv_VectorToRotator` (- (`GoMapBuilder.GetPosition` _returnvalue (`MapObstacleInterface.GetCoordinate` Target false)) (`GoMapBuilder.GetPosition` _returnvalue (`GoChessPawn.Coordinate` _array_element)))) _returnvalue_scale_2) true 0.0 0.125)
      (bind _asbp_go_chess_pawn_base (cast `/Game/GameCore/Blueprints/Chesses/BP_GoChessPawnBase` _array_element))
      (`self.PlayAnimMontage` _asbp_go_chess_pawn_base (`/Game/GameCore/Blueprints/Chesses/BP_GoChessPawnBase.OverrideAnimMontage` _asbp_go_chess_pawn_base) 1.0 "None"))
    (`ChessMovementComponent.MoveActorOnce` (`self.ChessMovementComponent`) (`KismetMathLibrary.MakeTransform` _returnvalue_location _returnvalue_rotation _returnvalue_scale) (`KismetMathLibrary.MakeTransform` _returnvalue_location (`KismetMathLibrary.Conv_VectorToRotator` (- (`GoMapBuilder.GetPosition` _returnvalue_2 (`MapObstacleInterface.GetCoordinate` Target false)) (`GoMapBuilder.GetPosition` _returnvalue_2 (`self.Coordinate`)))) _returnvalue_scale) true 0.0 0.125)
    (`|ExecutionSequence`
      (:`then_0`
        (bind _returnvalue_3 (`self.PlayAnimMontage` (`self.OverrideAnimMontage`)))
        (`KismetSystemLibrary.Delay` _returnvalue_3)
        (set `self.bIsLocallySelected` false)
        (`self.OnChangeOperationTransactionDelegate` "NotInTransaction")
        (bind _ashealth_notifier_interface (cast `HealthNotifierInterface` Target))
        (`HealthNotifierInterface.NotifyHealthViewToUpdate` _ashealth_notifier_interface)
        (`/Engine/EditorBlueprintResources/ActorMacros.Switch Has Authority`
          (:`Authority`
            (`KismetSystemLibrary.Delay` 1.0)
            (`MapObstacleInterface.DestroySelfIfNeeded` Target (`self.OwningPlayerIndex`))))))))

(fn `UserConstructionScript`)